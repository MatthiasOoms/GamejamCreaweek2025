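; Base enemy actor that attacks the player and takes damage from the player's slime trails and splatted slime balls.
; Capsule overlaps count trails and puddles underfoot, and Tick applies damage every frame, with trails taking priority.
; TakeDamage plays sound and animation, reduces health, then knocks the enemy backward without sweep or calls Die.
; Die removes it from every BP_EnemyManager array and destroys it.
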(event OnComponentBeginOverlap(CapsuleComponent)
  (params (OverlappedComponent :type Primitive%20Component%20Object%20Reference) (OtherActor :type Actor%20Object%20Reference) (OtherComp :type Primitive%20Component%20Object%20Reference) (OtherBodyIndex :type Integer) (bFromSweep :type Boolean) (SweepResult :type Hit%20Result%20Structure%20%28by%20ref%29))
  (Utilities|Casting|CastToBP_SlimeTrail OtherActor
    (:then
      (Math|Integer|IncrementInt (Variables|Default|GetStandingOnTrails)))
    (:CastFailed
      (bind _asbp_slim_ball (Utilities|Casting|CastToBP_SlimBall OtherActor))
      (if (Variables|/Game/Blueprints/Player/BP_SlimBall.BP_SlimBall_C|GetHasBecomeSplat _asbp_slim_ball)
        (Math|Integer|IncrementInt (Variables|Default|GetStandingOnPuddles))))))

(event OnComponentEndOverlap(CapsuleComponent)
  (params (OverlappedComponent :type Primitive%20Component%20Object%20Reference) (OtherActor :type Actor%20Object%20Reference) (OtherComp :type Primitive%20Component%20Object%20Reference) (OtherBodyIndex :type Integer))
  (Utilities|Casting|CastToBP_SlimeTrail OtherActor
    (:then
      (Math|Integer|DecrementInt (Variables|Default|GetStandingOnTrails)))
    (:CastFailed
      (bind _asbp_slim_ball (Utilities|Casting|CastToBP_SlimBall OtherActor))
      (if (Variables|/Game/Blueprints/Player/BP_SlimBall.BP_SlimBall_C|GetHasBecomeSplat _asbp_slim_ball)
        (Math|Integer|DecrementInt (Variables|Default|GetStandingOnPuddles))))))

(event EventTick
  (params (DeltaSeconds :type Float%20%28single-precision%29))
  (if (> (Variables|Default|GetStandingOnTrails) 0)
    (CallFunction|TakeDamage (Variables|Default|GetDamageTrail))
    (Development|PrintString "Hurt")
    (elif (> (Variables|Default|GetStandingOnPuddles) 0)
      (CallFunction|TakeDamage (Variables|Default|GetDamageBallPuddle))
      (Development|PrintString "Hurt"))))

(fn ConstructionScript)

(fn Attack
  (params (Player :type Actor%20Object%20Reference))
  (bind _asbp_player (Utilities|Casting|CastToBP_Player Player))
  (Default|DamagePlayer _asbp_player (Variables|Attack|GetDamage))
  (Components|Animation|PlayAnimation (Variables|Character|GetMesh) "/Game/ArtAssets/SkeletalMeshes/BaseCharacter/BaseCharRig_Anim_Attack_Generic.BaseCharRig_Anim_Attack_Generic" false)
  (Audio|SpawnSoundAttached "/Game/Audio/SFX/SC_EnemyAttack.SC_EnemyAttack" (Variables|Collision|GetCapsuleComponent) "None" "0, 0, 0" "0, 0, 0" "KeepRelativeOffset" false 1.0 1.0 0.0 0 0))

(fn TakeDamage
  (params (Amount :type Integer))
  (bind _knockbackdistance (Variables|Default|GetKnockbackDistance))
  (bind _capsulecomponent (Variables|Collision|GetCapsuleComponent))
  (bind _returnvalue (* _knockbackdistance -1.0))
  (Audio|SpawnSoundAttached "/Game/Audio/SFX/SC_EnemyDamage.SC_EnemyDamage" (Variables|Collision|GetCapsuleComponent) "None" "0, 0, 0" "0, 0, 0" "KeepRelativeOffset" false 1.0 1.0 0.0 0 0)
  (Components|Animation|PlayAnimation (Variables|Character|GetMesh) "/Game/ArtAssets/SkeletalMeshes/BaseCharacter/BaseCharRig_Anim_Damagei.BaseCharRig_Anim_Damagei" false)
  (bind _output_get (Variables|Default|SetHealth (- (Variables|Default|GetHealth) Amount)))
  (if (<= _output_get 0)
    (CallFunction|Die)
    (else
      (Transformation|SetWorldLocation _capsulecomponent (+ (Transformation|GetWorldLocation _capsulecomponent) (* (Math|Vector|GetForwardVector _capsulecomponent) (Math|Vector|MakeVector _returnvalue _returnvalue _returnvalue))) false false))))

(fn Die
  (Audio|SpawnSoundatLocation "/Game/Audio/SFX/SC_EnemyDies.SC_EnemyDies" (Transformation|GetActorLocation) "0, 0, 0" 1.0 1.0 0.0 0 0)
  ;[1 1 1] Revome Enemy from Enemy Manager
  (bind _outactors (Actor|GetAllActorsOfClass "/Game/Blueprints/Enemies/BP_EnemyManager.BP_EnemyManager_C"))
  (for _array_element _outactors
    (for _array_element_2 (Variables|/Game/Blueprints/Enemies/BP_EnemyManager.BP_EnemyManager_C|GetEnemyArray _array_element)
      (if (== _array_element_2 self)
        (Utilities|Array|RemoveItem (Variables|/Game/Blueprints/Enemies/BP_EnemyManager.BP_EnemyManager_C|GetEnemyArray _array_element) _array_element_2))))
  (Actor|DestroyActor))