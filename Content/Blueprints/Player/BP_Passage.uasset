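; BP_Passage is an overlap-driven actor that narrows the player's capsule while the player is inside it, presumably to fit through a tight passage.
; On begin overlap with a BP_Player, it caches the capsule's world Y scale in LastScale, then squashes that axis to a fixed fraction, leaving X and Z unchanged.
; On end overlap, it restores the cached Y scale.
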(event EventBeginPlay)

(event Collision|EventActorBeginOverlap
  (params (OtherActor :type Actor%20Object%20Reference))
  (bind _asbp_player (Utilities|Casting|CastToBP_Player OtherActor))
  (Variables|Default|SetLastScale (.y (Transformation|GetWorldScale (Variables|/Script/Engine.Character|GetCapsuleComponent _asbp_player))))
  (Transformation|SetWorldScale3D (Variables|/Script/Engine.Character|GetCapsuleComponent _asbp_player) (Math|Vector|MakeVector (.x (Transformation|GetWorldScale (Variables|/Script/Engine.Character|GetCapsuleComponent _asbp_player))) 0.25 (.z (Transformation|GetWorldScale (Variables|/Script/Engine.Character|GetCapsuleComponent _asbp_player))))))

(event EventTick
  (params (DeltaSeconds :type Float%20%28single-precision%29)))

(event Collision|EventActorEndOverlap
  (params (OtherActor :type Actor%20Object%20Reference))
  (bind _asbp_player (Utilities|Casting|CastToBP_Player OtherActor))
  (Transformation|SetWorldScale3D (Variables|/Script/Engine.Character|GetCapsuleComponent _asbp_player) (Math|Vector|MakeVector (.x (Transformation|GetWorldScale (Variables|/Script/Engine.Character|GetCapsuleComponent _asbp_player))) (Variables|Default|GetLastScale) (.z (Transformation|GetWorldScale (Variables|/Script/Engine.Character|GetCapsuleComponent _asbp_player))))))

(fn ConstructionScript)