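; Boss enemy with swing, dash and ranged attacks, each with a decal indicator, whose death pauses the game and opens the win menu.
; Attack functions damage players overlapping each attack's shape; ShowAttackUI moves the ranged decal and shape to a given location.
; DashAttack deals SwingAttackDamage immediately, then Tick lerps the boss with sweep to the overlapped player or a forward point.
; Tick also prints the forward vector when not dashing.
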(event EventBeginPlay
  (Variables|Dash|SetDashShapeDefaultLocation (Variables|/Script/Engine.SceneComponent|GetRelativeLocation (Variables|Default|GetDashAttackDecal)))
  (Variables|Default|SetHealth 100))

(event Collision|EventActorBeginOverlap
  (params (OtherActor :type Actor%20Object%20Reference)))

(event EventTick
  (params (DeltaSeconds :type Float%20%28single-precision%29))
  (if (Variables|Dash|GetIsDashing)
    ;[0.15 0.15 0.15 0.5] update dash time
    (bind _output_get (Variables|Dash|SetCurrentDashingTime (+ (Variables|Dash|GetCurrentDashingTime) DeltaSeconds)))
    ;[0.15 0.15 0.15 0.5] move actor
    (Transformation|SetActorLocation (Math|Vector|Lerp(Vector) (Variables|Dash|GetStartLocation) (Variables|Dash|GetTargetLocation) (/ _output_get (Variables|Dash|GetDashMovingTime))) true false)
    ;[0.15 0.15 0.15 0.5] check if stop dashing
    (if (>= (Variables|Dash|GetCurrentDashingTime) (Variables|Dash|GetDashMovingTime))
      (Variables|Dash|SetIsDashing false)
      (Utilities|FlowControl|Sequence))
    (else
      (Development|PrintString (Utilities|String|ToString(Vector) (Transformation|GetActorForwardVector))))))

(fn ConstructionScript)

(fn ShowAttackUI
  (params (AttackIndex :type Integer) (Location :type Vector))
  (bind _rangedattackdecal (Variables|Default|GetRangedAttackDecal))
  (switch int AttackIndex
    (:0
      (Rendering|SetVisibility (Variables|Default|GetSwingAttackDecal) true false))
    (:1
      (Rendering|SetVisibility (Variables|Default|GetDashAttackDecal) true false))
    (:2
      (Transformation|SetWorldLocation _rangedattackdecal Location false false)
      (Rendering|SetVisibility _rangedattackdecal true false))))

(fn HideAttackUI
  (params (AttackIndex :type Integer))
  (switch int AttackIndex
    (:Default
      (Utilities|FlowControl|Sequence
        (:then_0
          (Rendering|SetVisibility (Variables|Default|GetSwingAttackDecal) false false :!label _label))
        (:then_1
          (Rendering|SetVisibility (Variables|Default|GetDashAttackDecal) false false :!label _label_2))
        (:then_2
          (Rendering|SetVisibility (Variables|Default|GetRangedAttackDecal) false false :!label _label_3))))
    (:0
      (goto _label))
    (:1
      (goto _label_2))
    (:2
      (goto _label_3))))

(fn SwingAttack
  (Components|Animation|PlayAnimation (Variables|Character|GetMesh) "/Game/ArtAssets/SkeletalMeshes/Boss/BossRig_Anim_Attack_Generic.BossRig_Anim_Attack_Generic" false)
  (for _array_element (Collision|GetOverlappingActors (Variables|Default|GetSwingAttackShape) "/Game/Blueprints/Player/BP_Player.BP_Player_C" :!class /Script/Engine.PrimitiveComponent)
    (bind _asbp_player (Utilities|Casting|CastToBP_Player _array_element))
    (Default|DamagePlayer _asbp_player (Variables|Damage|GetSwingAttackDamage))))

(fn DashAttack
  (bind _dashattackshape (Variables|Default|GetDashAttackShape))
  (bind _overlappingactors (Collision|GetOverlappingActors _dashattackshape "/Game/Blueprints/Player/BP_Player.BP_Player_C" :!class /Script/Engine.PrimitiveComponent))
  (Variables|Dash|SetCurrentDashingTime 0.0)
  (Variables|Dash|SetIsDashing true)
  (Variables|Dash|SetStartLocation (Transformation|GetActorLocation))
  (if (Utilities|Array|IsEmpty _overlappingactors)
    (Variables|Dash|SetTargetLocation (+ (Variables|Dash|GetStartLocation) (* (Transformation|GetActorForwardVector) (Variables|Default|GetDashDistance))))
    (else
      (Variables|Dash|SetTargetLocation (Transformation|GetActorLocation (Utilities|Array|Get(acopy) _overlappingactors)))
      (for _array_element _overlappingactors
        (bind _asbp_player (Utilities|Casting|CastToBP_Player _array_element))
        (Default|DamagePlayer _asbp_player (Variables|Damage|GetSwingAttackDamage))))))

(fn RangedAttack
  (for _array_element (Collision|GetOverlappingActors (Variables|Default|GetRangedAttackShape) "/Game/Blueprints/Player/BP_Player.BP_Player_C" :!class /Script/Engine.PrimitiveComponent)
    (bind _asbp_player (Utilities|Casting|CastToBP_Player _array_element))
    (Default|DamagePlayer _asbp_player (Variables|Damage|GetRangedAttackDamage))))

(fn StartAttackAnimation
  (params (AttackIndex :type Integer))
  (switch int AttackIndex
    (:1
      (Components|Animation|PlayAnimation (Variables|Character|GetMesh) "/Game/ArtAssets/SkeletalMeshes/Boss/BossRig_Anim_Boss_MainAttack.BossRig_Anim_Boss_MainAttack" false))
    (:2
      (Components|Animation|PlayAnimation (Variables|Character|GetMesh) "/Game/ArtAssets/SkeletalMeshes/Boss/BossRig_Anim_Boss_Magic.BossRig_Anim_Boss_Magic" false))))

(fn Die
  (Game|SetGamePaused true)
  (Game|OpenLevel(byObjectReference) "/Game/Scene/WinMenu.WinMenu")
  (|CallParentFunction))