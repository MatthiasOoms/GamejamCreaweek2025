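; Player controller that turns Enhanced Input into BP_Player actions: movement, aiming, absorbing, slime shooting and pausing.
; Movement follows control rotation, aiming applies yaw only, absorb calls EatAll while overlapping, and pause opens a menu widget.
; Holding shoot scales force by hold time and moves a reused landing marker via projectile path prediction.
; Releasing hides the marker and spawns a BP_SlimBall with that force.
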(event Input|EnhancedActionEvents|EnhancedInputActionIA_Movement
  (params (ActionValue :type Vector%202D%20Structure) (ElapsedSeconds :type Float%20%28double-precision%29) (TriggeredSeconds :type Float%20%28double-precision%29) (InputAction :type Input%20Action%20Object%20Reference :default "/Game/Input/Actions/IA_Movement.IA_Movement"))
  ;[0.15 0.15 0.15 0.5] Movement
  (bind _asbp_player (Utilities|Casting|CastToBP_Player (Pawn|GetControlledPawn)))
  (Pawn|Input|AddMovementInput _asbp_player (Math|Vector|RotateVector (Math|Vector|MakeVector (.y ActionValue) (.x ActionValue) 0.0) (Pawn|GetControlRotation :!class /Script/Engine.Controller)) 1.0 false))

(event Input|EnhancedActionEvents|EnhancedInputActionIA_Aim
  (params (ActionValue :type Vector%202D%20Structure) (ElapsedSeconds :type Float%20%28double-precision%29) (TriggeredSeconds :type Float%20%28double-precision%29) (InputAction :type Input%20Action%20Object%20Reference :default "/Game/Input/Actions/IA_Aim.IA_Aim"))
  (bind _returnvalue (Pawn|GetControlledPawn))
  ;[0.15 0.15 0.15 0.5] Aiming
  (bind _asbp_player (Utilities|Casting|CastToBP_Player _returnvalue))
  (Pawn|SetControlRotation (Pawn|GetController _asbp_player) (Math|Rotator|CombineRotators (Math|Rotator|MakeRotator 0.0 0.0 (* (.x ActionValue) (Variables|Default|GetRotationSpeed) 1.0)) (Transformation|GetActorRotation _returnvalue))))

(event Input|EnhancedActionEvents|EnhancedInputActionIA_Absorb
  (params (ActionValue :type Boolean) (ElapsedSeconds :type Float%20%28double-precision%29) (TriggeredSeconds :type Float%20%28double-precision%29) (InputAction :type Input%20Action%20Object%20Reference :default "/Game/Input/Actions/IA_Absorb.IA_Absorb"))
  (bind _asbp_player (Utilities|Casting|CastToBP_Player (Pawn|GetControlledPawn)))
  (if (Variables|/Game/Blueprints/Player/BP_Player.BP_Player_C|GetIsOverlapping _asbp_player)
    (Default|EatAll _asbp_player)))

(event Input|EnhancedActionEvents|EnhancedInputActionIA_Shoot
  (params (ActionValue :type Boolean) (ElapsedSeconds :type Float%20%28double-precision%29) (TriggeredSeconds :type Float%20%28double-precision%29) (InputAction :type Input%20Action%20Object%20Reference :default "/Game/Input/Actions/IA_Shoot.IA_Shoot"))
  (bind _returnvalue (Game|Player|GetPlayerPawn 0))
  (bind _returnvalue_2 (Game|Player|GetPlayerPawn 0))
  (:Triggered
    (bind _asbp_slim_ball (Utilities|Casting|CastToBP_SlimBallClass "/Game/Blueprints/Player/BP_SlimBall.BP_SlimBall_C"))
    (bind _asbp_player (Utilities|Casting|CastToBP_Player (Game|Player|GetPlayerPawn 0)))
    (bind _outhit (Class|GameplayStatics|BlueprintPredictProjectilePathbyTraceChannel (Transformation|GetWorldLocation (Variables|/Game/Blueprints/Player/BP_Player.BP_Player_C|GetSlimeBallSpawnPoint _asbp_player)) (* (Math|Vector|RotateVectorAroundAxis (Transformation|GetActorForwardVector _returnvalue) (.Angle (Utilities|GetClassDefaults _asbp_slim_ball)) (Transformation|GetActorRightVector _returnvalue)) (* TriggeredSeconds (Variables|Default|GetForceIncreaseScaler))) true 1.0 "ECC_WorldDynamic" false 0 "None"))
    (Utilities|IsValid (Variables|Default|GetHitPoint)
      (:Is%20Valid
        (Rendering|SetActorHiddenInGame (Variables|Default|GetHitPoint) false)
        (Transformation|SetActorLocation (Variables|Default|GetHitPoint) (.Location (Collision|BreakHitResult _outhit)) false true))
      (:Is%20Not%20Valid
        (bind _returnvalue_3 (Game|SpawnActorfromClass "/Game/Blueprints/Player/BP_PredictedPosition.BP_PredictedPosition_C" (Math|Transform|MakeTransform (.Location (Collision|BreakHitResult _outhit)) "0, 0, 0" "1.000000,1.000000,1.000000") "Undefined" "MultiplyWithRoot" 0 0))
        (Variables|Default|SetHitPoint _returnvalue_3))))
  (:Completed
    (Rendering|SetActorHiddenInGame (Variables|Default|GetHitPoint) true)
    (bind _asbp_player_2 (Utilities|Casting|CastToBP_Player _returnvalue_2))
    (bind _returnvalue_4 (Game|SpawnActorfromClass "/Game/Blueprints/Player/BP_SlimBall.BP_SlimBall_C" (Math|Transform|MakeTransform (Transformation|GetWorldLocation (Variables|/Game/Blueprints/Player/BP_Player.BP_Player_C|GetSlimeBallSpawnPoint _asbp_player_2)) (.rotation (Transformation|GetActorTransform _returnvalue_2)) "1.000000,1.000000,1.000000") "AlwaysSpawn" "MultiplyWithRoot" 0 0))
    (Variables|/Game/Blueprints/Player/BP_SlimBall.BP_SlimBall_C|SetForce _returnvalue_4 (* TriggeredSeconds (Variables|Default|GetForceIncreaseScaler)))))

(event Input|EnhancedActionEvents|EnhancedInputActionIA_Pause
  (params (ActionValue :type Boolean) (ElapsedSeconds :type Float%20%28double-precision%29) (TriggeredSeconds :type Float%20%28double-precision%29) (InputAction :type Input%20Action%20Object%20Reference :default "/Game/Input/Actions/IA_Pause.IA_Pause"))
  (bind _returnvalue (UserInterface|CreateWidget "/Game/Blueprints/MenuWidgets/BPW_PauseMenu.BPW_PauseMenu_C"))
  (UserInterface|Viewport|AddtoViewport _returnvalue 0)
  (Game|SetGamePaused true))

(fn ConstructionScript)