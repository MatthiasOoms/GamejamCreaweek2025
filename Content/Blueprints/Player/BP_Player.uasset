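; Player slime whose body size tracks its health, shrinking on damage and growing on healing, with death reloading the current level.
; A collision sphere collects overlapping BP_Absorbable actors, which Tick absorbs with a sound while IsEatingAbsorbable is set.
; Tick also animates blinking by scaling both eyes on timers and spawns randomly scattered, rotated and scaled BP_SlimeTrail actors whenever the spawn point moves past a set distance.
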(event OnComponentBeginOverlap(SphereCollision)
  (params (OverlappedComponent :type Primitive%20Component%20Object%20Reference) (OtherActor :type Actor%20Object%20Reference) (OtherComp :type Primitive%20Component%20Object%20Reference) (OtherBodyIndex :type Integer) (bFromSweep :type Boolean) (SweepResult :type Hit%20Result%20Structure%20%28by%20ref%29))
  (bind _asbp_absorbable (Utilities|Casting|CastToBP_Absorbable OtherActor))
  (Utilities|Array|Add (Variables|Absorb|GetAbsorbableRef) _asbp_absorbable)
  (Variables|Absorb|SetIsOverlapping true))

(event OnComponentEndOverlap(SphereCollision)
  (params (OverlappedComponent :type Primitive%20Component%20Object%20Reference) (OtherActor :type Actor%20Object%20Reference) (OtherComp :type Primitive%20Component%20Object%20Reference) (OtherBodyIndex :type Integer))
  (bind _asbp_absorbable (Utilities|Casting|CastToBP_Absorbable OtherActor))
  (Utilities|Array|RemoveItem (Variables|Absorb|GetAbsorbableRef) _asbp_absorbable)
  (Variables|Absorb|SetIsOverlapping false))

(event Custom|DamagePlayer
  (params (DamageAmount :type Integer))
  ;[1 0 0 0.5] Damage Player for X amount
  ;;[1 1 1] Damage is positive
  (if (>= DamageAmount 0)
    ;;[1 1 1] New health is not negative
    (if (>= (- (Variables|Health|GetCurrentHealth) DamageAmount) 0)
      ;;[1 1 1] Set to new health or 0
      (Variables|Health|SetCurrentHealth (- (Variables|Health|GetCurrentHealth) DamageAmount))
      ;;[1 1 1] Change player radius
      (Transformation|SetWorldScale3D (Variables|Collision|GetCapsuleComponent) (Math|Vector|MakeVector (+ (/ (Variables|Health|GetCurrentHealth) (Variables|Health|GetMaxHealth)) (Variables|Size|GetMinScale)) (+ (/ (Variables|Health|GetCurrentHealth) (Variables|Health|GetMaxHealth)) (Variables|Size|GetMinScale)) (+ (/ (Variables|Health|GetCurrentHealth) (Variables|Health|GetMaxHealth)) (Variables|Size|GetMinScale))))
      ;;[1 1 1] Play SFX
      (bind _newparam1 (CallFunction|PlaySFX "/Game/Audio/SFX/SC_SlimeHurt.SC_SlimeHurt"))
      (Utilities|FlowControl|Delay 1.0)
      (Audio|Components|Audio|Stop _newparam1)
      (else
        (Variables|Health|SetCurrentHealth 0)
        ;;[1 1 1] Player Death
        (CallFunction|Death)))))

(event Custom|HealPlayer
  (params (Heal%20Amount :type Integer))
  ;[1 0 0 0.5] Healing Player for X amount
  ;;[1 1 1] Healing is positive
  (if (> Heal%20Amount 0)
    ;;[1 1 1] New health is not over max
    (if (< (+ (Variables|Health|GetCurrentHealth) Heal%20Amount) (Variables|Health|GetMaxHealth))
      ;;[1 1 1] Set to new health or max
      (Variables|Health|SetCurrentHealth (+ (Variables|Health|GetCurrentHealth) Heal%20Amount))
      (else
        (Variables|Health|SetCurrentHealth (Variables|Health|GetMaxHealth))))
    ;;[1 1 1] Change player radius
    (Transformation|SetWorldScale3D (Variables|Collision|GetCapsuleComponent) (Math|Vector|MakeVector (+ (/ (Variables|Health|GetCurrentHealth) (Variables|Health|GetMaxHealth)) (Variables|Size|GetMinScale)) (+ (/ (Variables|Health|GetCurrentHealth) (Variables|Health|GetMaxHealth)) (Variables|Size|GetMinScale)) (+ (/ (Variables|Health|GetCurrentHealth) (Variables|Health|GetMaxHealth)) (Variables|Size|GetMinScale))))))

(event Custom|Death
  ;[0.15 0.15 0.15 0.5] Implement Death Functionality
  (bind _returnvalue (Game|GetCurrentLevelName true))
  (Game|OpenLevel(byName) (Utilities|String|StringToName _returnvalue)))

(event EventBeginPlay
  ;[0.15 0.15 0.15 0.5] Set current health to max health
  (bind _output_get (Variables|Health|SetCurrentHealth (Variables|Health|GetMaxHealth)))
  ;[0.15 0.15 0.15 0.5] Set minimum player scale
  (Variables|Size|SetMinScale (/ _output_get (* 1.5 1e+02)))
  ;[0.15 0.15 0.15 0.5] Change player radius
  (Transformation|SetWorldScale3D (Variables|Collision|GetCapsuleComponent) (Math|Vector|MakeVector (+ (/ (Variables|Health|GetCurrentHealth) (Variables|Health|GetMaxHealth)) (Variables|Size|GetMinScale)) (+ (/ (Variables|Health|GetCurrentHealth) (Variables|Health|GetMaxHealth)) (Variables|Size|GetMinScale)) (+ (/ (Variables|Health|GetCurrentHealth) (Variables|Health|GetMaxHealth)) (Variables|Size|GetMinScale))))
  ;[0.15 0.15 0.15 0.5] Set initial scale of eyes
  (bind _output_get_2 (Variables|Blink|SetInitialScaleRightEye (Variables|/Script/Engine.SceneComponent|GetRelativeScale3D (Variables|Default|GetEyeRight))))
  (Variables|Blink|SetInitialScaleLeftEye _output_get_2))

(event EventTick
  (params (DeltaSeconds :type Float%20%28single-precision%29))
  (bind _trailscatter (Variables|Trail|GetTrailScatter))
  (bind _trailrotation (Variables|Trail|GetTrailRotation))
  (bind _trailminscale (Variables|Trail|GetTrailMinScale))
  (bind _trailmaxscale (Variables|Trail|GetTrailMaxScale))
  (bind _trailspawnpoint (Variables|Default|GetTrailSpawnPoint))
  (bind _returnvalue (Transformation|GetWorldLocation _trailspawnpoint))
  (bind _returnvalue_2 (Math|Random|RandomFloatinRange _trailminscale _trailmaxscale))
  (bind _returnvalue_3 (* _trailscatter -1.0))
  (Utilities|FlowControl|Sequence
    (:then_0
      ;[0.15 0.15 0.15 0.5] Absorbable
      (if (Variables|Absorb|GetIsEatingAbsorbable)
        (for _array_element (Variables|Absorb|GetAbsorbableRef)
          (Default|AbsorbedObject _array_element)
          (CallFunction|PlaySFX "/Game/Audio/SFX/SC_Absorb.SC_Absorb")
          (Utilities|Array|RemoveItem (Variables|Absorb|GetAbsorbableRef) _array_element))))
    (:then_1
      (CallFunction|Blink DeltaSeconds))
    (:then_2
      (if (> (Math|Vector|Distance(Vector) (Variables|Trail|GetLastTrailPos) _returnvalue) (Variables|Trail|GetTrailInterval))
        (bind _returnvalue_4 (Game|SpawnActorfromClass "/Game/Blueprints/Player/BP_SlimeTrail.BP_SlimeTrail_C" (Math|Transform|MakeTransform (+ _returnvalue (Math|Vector|MakeVector (Math|Random|RandomFloatinRange _returnvalue_3 _trailscatter) (Math|Random|RandomFloatinRange _returnvalue_3 _trailscatter) 0.0)) (Math|Rotator|MakeRotator 0.0 0.0 (Math|Random|RandomFloatinRange (* _trailrotation -1.0) _trailrotation)) (Math|Vector|MakeVector 0.1 _returnvalue_2 _returnvalue_2)) "AdjustIfPossibleButDontSpawnIfColliding" "MultiplyWithRoot" 0 0))
        (Variables|Trail|SetLastTrailPos (Transformation|GetWorldLocation (Variables|/Script/Engine.Actor|GetRootComponent _returnvalue_4)))))))

(fn ConstructionScript)

(fn Blink
  (params (InputPin :type Float%20%28single-precision%29))
  (if (Variables|Blink|GetBlinkCooldown)
    (Variables|Blink|SetBlinkCooldownTimer (+ InputPin (Variables|Blink|GetBlinkCooldownTimer)))
    (if (> (Variables|Blink|GetBlinkCooldownTimer) 3.0)
      (Variables|Blink|SetBlinkCooldown false))
    (else
      (Variables|Blink|SetBlinkCooldownTimer 0.0)
      (if (Variables|Blink|GetAreEyesOpen)
        (Variables|Blink|SetBlinkTimer (- (Variables|Blink|GetBlinkTimer) InputPin))
        (Transformation|SetRelativeScale3D (Variables|Default|GetEyeRight) (- (Variables|Blink|GetInitialScaleRightEye) (Math|Vector|MakeVector 0.0 0.0 (Variables|Blink|GetBlinkTimer))))
        (Transformation|SetRelativeScale3D (Variables|Default|GetEyeLeft) (- (Variables|Blink|GetInitialScaleLeftEye) (Math|Vector|MakeVector 0.0 0.0 (Variables|Blink|GetBlinkTimer))))
        (if (< (Variables|Blink|GetBlinkTimer) 0.5)
          (Variables|Blink|SetAreEyesOpen false)
          (if (Variables|Blink|GetAreEyesOpen) :!label _label
            (Variables|Blink|SetBlinkCooldown true)))
        (else
          (Variables|Blink|SetBlinkTimer (+ (Variables|Blink|GetBlinkTimer) InputPin))
          (Transformation|SetRelativeScale3D (Variables|Default|GetEyeRight) (- (Variables|Blink|GetInitialScaleRightEye) (Math|Vector|MakeVector 0.0 0.0 (Variables|Blink|GetBlinkTimer))))
          (Transformation|SetRelativeScale3D (Variables|Default|GetEyeLeft) (- (Variables|Blink|GetInitialScaleLeftEye) (Math|Vector|MakeVector 0.0 0.0 (Variables|Blink|GetBlinkTimer))))
          (if (> (Variables|Blink|GetBlinkTimer) 1.0)
            (Variables|Blink|SetAreEyesOpen true)
            (goto _label)))))))

(fn PlaySFX
  (params (NewParam :type Sound%20Base%20Object%20Reference))
  (bind _returnvalue (Audio|SpawnSoundAttached NewParam (Variables|Collision|GetCapsuleComponent) "None" "0, 0, 0" "0, 0, 0" "KeepRelativeOffset" false 1.0 1.0 0.0 0 0))
  (return _returnvalue))