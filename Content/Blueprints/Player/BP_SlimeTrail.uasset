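; BP_SlimeTrail is a player slime trail actor that shrinks away over its lifetime and then removes itself.
; Tick accumulates a timer and uniformly sets the root's world scale to the remaining fraction of Lifetime, giving a linear shrink from full size.
; The actor destroys itself once that fraction drops below zero.
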(event EventBeginPlay)

(event Collision|EventActorBeginOverlap
  (params (OtherActor :type Actor%20Object%20Reference)))

(event EventTick
  (params (DeltaSeconds :type Float%20%28single-precision%29))
  (bind _output_get (Variables|Default|SetTimer (+ DeltaSeconds (Variables|Default|GetTimer))))
  (Transformation|SetWorldScale3D (Variables|Default|GetDefaultSceneRoot) (Math|Vector|MakeVector (- 1.0 (/ _output_get (Variables|Default|GetLifetime))) (- 1.0 (/ _output_get (Variables|Default|GetLifetime))) (- 1.0 (/ _output_get (Variables|Default|GetLifetime)))))
  (if (< (- 1.0 (/ _output_get (Variables|Default|GetLifetime))) 0.0)
    (Actor|DestroyActor)))

(fn ConstructionScript)