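; AI controller for base enemies that runs the BT_BaseEnemy behavior tree and seeds its Blackboard.
; On possess it starts the tree, then writes the attack range, interest (move-to-player) range and time between attacks from its own variables, using key-name variables.
; On BeginPlay it finds the BP_Player actor by class and stores it as the player key.
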(event EventBeginPlay
  ;[1 1 1] set player
  (bind _returnvalue (Actor|GetActorOfClass "/Game/Blueprints/Player/BP_Player.BP_Player_C"))
  (AI|Components|Blackboard|SetValueasObject (Variables|Default|GetBlackboard) (Variables|Default|GetPlayerKeyName) _returnvalue))

(event EventTick
  (params (DeltaSeconds :type Float%20%28single-precision%29)))

(event EventPossess
  (params (PossessedPawn :type Pawn%20Object%20Reference))
  ;[1 1 1] starts bavior tree execution
  (AI|RunBehaviorTree "/Game/AI/BT_BaseEnemy.BT_BaseEnemy")
  ;[0.15 0.15 0.15 0.5] set attack range
  (AI|Components|Blackboard|SetValueasFloat (Variables|Default|GetBlackboard) (Variables|Default|GetAttackRangeKeyName) (Variables|Default|GetAttackRange))
  ;[0.15 0.15 0.15 0.5] set move to player range
  (AI|Components|Blackboard|SetValueasFloat (Variables|Default|GetBlackboard) (Variables|Default|GetInterestRangeKeyName) (Variables|Default|GetInterestRange))
  ;[0.15 0.15 0.15 0.5] set attack rate
  (AI|Components|Blackboard|SetValueasFloat (Variables|Default|GetBlackboard) (Variables|Default|GetTimeBetweenAttacksKeyName) (Variables|Default|GetTimeBetweenAttacks)))

(fn ConstructionScript)