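; BP_SlimBall is a physics-driven ball actor that launches itself along an angled arc relative to the player pawn's facing.
; On its first Tick, guarded by a HasFired flag, it rotates player 0's forward vector around that pawn's right vector by Angle.
; It multiplies the result by Force and sets it as the Ball component's linear velocity, leaving the flight to physics.
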(event EventBeginPlay)

(event Collision|EventActorBeginOverlap
  (params (OtherActor :type Actor%20Object%20Reference)))

(event EventTick
  (params (DeltaSeconds :type Float%20%28single-precision%29))
  (bind _returnvalue (Game|Player|GetPlayerPawn 0))
  (if (not (Variables|Default|GetHasFired))
    (Variables|Default|SetHasFired true)
    (Physics|SetPhysicsLinearVelocity (Variables|Default|GetBall) (* (Math|Vector|RotateVectorAroundAxis (Transformation|GetActorForwardVector _returnvalue) (Variables|Default|GetAngle) (Transformation|GetActorRightVector _returnvalue)) (Variables|Default|GetForce)) false "None")))

(fn ConstructionScript)