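; Test player Blueprint whose body size reflects health, with absorbing of nearby objects and animated blinking eyes.
; Damage and healing events update health and rescale the capsule above a minimum offset; Death is an empty stub.
; Sphere overlaps track BP_Absorbable actors, which Tick absorbs while IsEatingAbsorbable is set; the power-up cast leads nowhere.
; Tick also animates blinking by varying eye Z scale, with a cooldown between blinks.
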(event OnComponentBeginOverlap(SphereCollision)
  (params (OverlappedComponent :type Primitive%20Component%20Object%20Reference) (OtherActor :type Actor%20Object%20Reference) (OtherComp :type Primitive%20Component%20Object%20Reference) (OtherBodyIndex :type Integer) (bFromSweep :type Boolean) (SweepResult :type Hit%20Result%20Structure%20%28by%20ref%29))
  (Utilities|FlowControl|Sequence
    (:then_0
      (bind _asbp_absorbable (Utilities|Casting|CastToBP_Absorbable OtherActor))
      (Utilities|Array|Add (Variables|Default|GetAbsorbableRef) _asbp_absorbable)
      (Variables|Default|SetIsOverlapping true))
    (:then_1
      (Utilities|Casting|CastToBP_PowerUp OtherActor))))

(event OnComponentEndOverlap(SphereCollision)
  (params (OverlappedComponent :type Primitive%20Component%20Object%20Reference) (OtherActor :type Actor%20Object%20Reference) (OtherComp :type Primitive%20Component%20Object%20Reference) (OtherBodyIndex :type Integer))
  (bind _asbp_absorbable (Utilities|Casting|CastToBP_Absorbable OtherActor))
  (Utilities|Array|RemoveItem (Variables|Default|GetAbsorbableRef) _asbp_absorbable)
  (Variables|Default|SetIsOverlapping false))

(event Custom|DamagePlayer
  (params (DamageAmount :type Integer))
  ;[1 0 0 0.5] Damage Player for X amount
  ;;[1 1 1] Damage is positive
  (if (>= DamageAmount 0)
    ;;[1 1 1] New health is not negative
    (if (>= (- (Variables|Health|GetCurrentHealth) DamageAmount) 0)
      ;;[1 1 1] Set to new health or 0
      (Variables|Health|SetCurrentHealth (- (Variables|Health|GetCurrentHealth) DamageAmount))
      ;;[1 1 1] Change player radius
      (Transformation|SetWorldScale3D (Variables|Collision|GetCapsuleComponent) (Math|Vector|MakeVector (+ (/ (Variables|Health|GetCurrentHealth) (Variables|Health|GetMaxHealth)) (Variables|Size|GetMinScale)) (+ (/ (Variables|Health|GetCurrentHealth) (Variables|Health|GetMaxHealth)) (Variables|Size|GetMinScale)) (+ (/ (Variables|Health|GetCurrentHealth) (Variables|Health|GetMaxHealth)) (Variables|Size|GetMinScale))))
      (else
        (Variables|Health|SetCurrentHealth 0)
        ;;[0.15 0.15 0.15 0.5] Player Death
        (CallFunction|Death)))))

(event Custom|HealPlayer
  (params (Heal%20Amount :type Integer))
  ;[1 0 0 0.5] Healing Player for X amount
  ;;[1 1 1] Healing is positive
  (if (> Heal%20Amount 0)
    ;;[1 1 1] New health is not over max
    (if (< (+ (Variables|Health|GetCurrentHealth) Heal%20Amount) (Variables|Health|GetMaxHealth))
      ;;[1 1 1] Set to new health or max
      (Variables|Health|SetCurrentHealth (+ (Variables|Health|GetCurrentHealth) Heal%20Amount))
      (else
        (Variables|Health|SetCurrentHealth (Variables|Health|GetMaxHealth))))
    ;;[1 1 1] Change player radius
    (Transformation|SetWorldScale3D (Variables|Collision|GetCapsuleComponent) (Math|Vector|MakeVector (+ (/ (Variables|Health|GetCurrentHealth) (Variables|Health|GetMaxHealth)) (Variables|Size|GetMinScale)) (+ (/ (Variables|Health|GetCurrentHealth) (Variables|Health|GetMaxHealth)) (Variables|Size|GetMinScale)) (+ (/ (Variables|Health|GetCurrentHealth) (Variables|Health|GetMaxHealth)) (Variables|Size|GetMinScale))))))

(event Custom|Death
  ;[0.15 0.15 0.15 0.5] Implement Death Functionality
)

(event EventBeginPlay
  ;[0.15 0.15 0.15 0.5] Set current health to max health
  (bind _output_get (Variables|Health|SetCurrentHealth (Variables|Health|GetMaxHealth)))
  ;[0.15 0.15 0.15 0.5] Set minimum player scale
  (Variables|Size|SetMinScale (/ _output_get (* 1.5 1e+02)))
  ;[0.15 0.15 0.15 0.5] Change player radius
  (Transformation|SetWorldScale3D (Variables|Collision|GetCapsuleComponent) (Math|Vector|MakeVector (+ (/ (Variables|Health|GetCurrentHealth) (Variables|Health|GetMaxHealth)) (Variables|Size|GetMinScale)) (+ (/ (Variables|Health|GetCurrentHealth) (Variables|Health|GetMaxHealth)) (Variables|Size|GetMinScale)) (+ (/ (Variables|Health|GetCurrentHealth) (Variables|Health|GetMaxHealth)) (Variables|Size|GetMinScale))))
  ;[0.15 0.15 0.15 0.5] Set initial scale of eyes
  (bind _output_get_2 (Variables|Default|SetInitialScaleRightEye (Variables|/Script/Engine.SceneComponent|GetRelativeScale3D (Variables|Default|GetEyeRight))))
  (Variables|Default|SetInitialScaleLeftEye _output_get_2))

(event EventTick
  (params (DeltaSeconds :type Float%20%28single-precision%29))
  (Utilities|FlowControl|Sequence
    (:then_0
      (if (Variables|Default|GetIsEatingAbsorbable)
        (for _array_element (Variables|Default|GetAbsorbableRef)
          (Default|AbsorbedObject _array_element)
          (Utilities|Array|RemoveItem (Variables|Default|GetAbsorbableRef) _array_element))))
    (:then_1
      (if (Variables|Default|GetBlinkCooldown)
        (Variables|Default|SetBlinkCooldownTimer (+ DeltaSeconds (Variables|Default|GetBlinkCooldownTimer)))
        (if (> (Variables|Default|GetBlinkCooldownTimer) 3.0)
          (Variables|Default|SetBlinkCooldown false))
        (else
          (Variables|Default|SetBlinkCooldownTimer 0.0)
          (if (Variables|Default|GetAreEyesOpen)
            (Variables|Default|SetBlinkTimer (- (Variables|Default|GetBlinkTimer) DeltaSeconds))
            (Transformation|SetRelativeScale3D (Variables|Default|GetEyeRight) (- (Variables|Default|GetInitialScaleRightEye) (Math|Vector|MakeVector 0.0 0.0 (Variables|Default|GetBlinkTimer))))
            (Transformation|SetRelativeScale3D (Variables|Default|GetEyeLeft) (- (Variables|Default|GetInitialScaleLeftEye) (Math|Vector|MakeVector 0.0 0.0 (Variables|Default|GetBlinkTimer))))
            (if (< (Variables|Default|GetBlinkTimer) 0.5)
              (Variables|Default|SetAreEyesOpen false)
              (if (Variables|Default|GetAreEyesOpen) :!label _label
                (Variables|Default|SetBlinkCooldown true)))
            (else
              (Variables|Default|SetBlinkTimer (+ (Variables|Default|GetBlinkTimer) DeltaSeconds))
              (Transformation|SetRelativeScale3D (Variables|Default|GetEyeRight) (- (Variables|Default|GetInitialScaleRightEye) (Math|Vector|MakeVector 0.0 0.0 (Variables|Default|GetBlinkTimer))))
              (Transformation|SetRelativeScale3D (Variables|Default|GetEyeLeft) (- (Variables|Default|GetInitialScaleLeftEye) (Math|Vector|MakeVector 0.0 0.0 (Variables|Default|GetBlinkTimer))))
              (if (> (Variables|Default|GetBlinkTimer) 1.0)
                (Variables|Default|SetAreEyesOpen true)
                (goto _label)))))))))

(fn ConstructionScript)